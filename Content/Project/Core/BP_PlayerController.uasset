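; Player controller for a multiplayer text chat, creating the chat and hint widgets on non-authority clients at BeginPlay.
; The Chat input action focuses the chat widget and switches between UI-only and game-only input, while Q removes the hint.
; SSend forwards messages to ThirdPersonGameMode for broadcast to all players, and TextToChat pushes received messages into the chat widget.
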(event Custom|ShowChatEvent
  (params (Focused :type Boolean))
  (bind _self self)
  (bind _widget_chat (Variables|Default|GetWidget_chat))
  ;[1 1 1] запускаем событие на фокус картеки в чат
  ; меняем инпут мод в зависимости от фокуса каретки
  (Default|ChatFocus _widget_chat Focused)
  (if Focused
    (Input|SetInputModeUIOnly _self _widget_chat "DoNotLock")
    (else
      (Input|SetInputModeGameOnly _self))))

(event Custom|SSend
  (params (Owner :type String) (TextOfMessage :type String))
  ;[1 1 1] Отправляем текст сообщения в гейммод
  (bind _asthird_person_game_mode (Utilities|Casting|CastToThirdPersonGameMode (Game|GetGameMode)))
  (Default|SendMessagetoAll _asthird_person_game_mode Owner TextOfMessage))

(event Custom|TextToChat
  (params (Owner :type String) (TextOfMessage :type String))
  ;[1 1 1] Переносим сообщение каждому игроку в виджет чата
  (Default|MessegetoArray (Variables|Default|GetWidget_chat) Owner TextOfMessage))

(event Custom|CreateChatWidget
  ;[1 1 1] Создаём виджет мультикастом и выводим его на Viewport
  (Networking|SwitchHasAuthority
    (:Remote
      (Utilities|FlowControl|Sequence
        (:then_0
          (bind _returnvalue (UserInterface|CreateWidget "/Game/ThirdPersonBP/Widget/WBP_chat.WBP_chat_C"))
          (bind _output_get (Variables|Default|SetWidget_chat _returnvalue))
          (UserInterface|Viewport|AddtoViewport _output_get 0))
        (:then_1
          (bind _returnvalue_2 (UserInterface|CreateWidget "/Game/ThirdPersonBP/Widget/WBP_Info.WBP_Info_C"))
          (bind _output_get_2 (Variables|Default|SetWidget_Info _returnvalue_2))
          (UserInterface|Viewport|AddtoViewport _output_get_2 0))))))

(event EventTick
  (params (DeltaSeconds :type Float%20%28single-precision%29)))

(event EventBeginPlay
  ;[1 1 1] Запускаем ивент создания чата в начале игры
  (CallFunction|CreateChatWidget))

(event Input|ActionEvents|InputActionChat
  (params (Key :type Key%20Structure :default "None"))
  ;[1 1 1] При нажатии действия "чат" (по умолчанию Enter) запускается ивент, позволяющий писать в чат
  (:Pressed
    (CallFunction|ShowChatEvent true)))

(event Input|KeyboardEvents|Q
  (params (Key :type Key%20Structure :default "None"))
  ;[1 1 1] Удаляем подсказку
  (:Pressed
    (Widget|RemovefromParent (Variables|Default|GetWidget_Info))))

(fn ConstructionScript)